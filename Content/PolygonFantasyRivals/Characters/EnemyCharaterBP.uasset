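; Enemy character Blueprint that dies when its capsule is overlapped by a spell actor derived from SpellParent.
; On a hit it turns the mesh into a physics ragdoll, disables movement and marks itself dead.
; After a short delay it asks its stored spawner, passed in through a setter event, to respawn at the capsule's transform, then destroys itself.
; Non-spell overlaps only print a debug string.
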(event `self.ReceiveBeginPlay`)

(event `get spawner`
  (params (spawner :type "/Game/PolygonFantasyRivals/Characters/Spawner Object Reference"))
  (set `self.spawner` spawner))

(event `ragdoll`
  ;[1 1 1] Ragdoll
  (`PrimitiveComponent.SetSimulatePhysics` (`self.Mesh`) true)
  (`CharacterMovementComponent.DisableMovement` (`self.CharacterMovement`)))

(event `self.CapsuleComponent.OnComponentBeginOverlap`
  (params (OverlappedComponent :type "PrimitiveComponent Object Reference") (OtherActor :type "Actor Object Reference") (OtherComp :type "PrimitiveComponent Object Reference") (OtherBodyIndex :type Integer) (bFromSweep :type Boolean) (SweepResult :type "HitResult Structure (by ref)"))
  (if (`KismetMathLibrary.ClassIsChildOf` (`GameplayStatics.GetObjectClass` OtherActor) "/Game/VirtualRealityBP/Blueprints/Spells/SpellParent.SpellParent_C")
    (`self.ragdoll`)
    (set `self.dead` true)
    (`KismetSystemLibrary.Delay` 3.0)
    (`/Game/PolygonFantasyRivals/Characters/Spawner.respawn` (`self.spawner`) (`SceneComponent.K2_GetComponentToWorld` (`self.CapsuleComponent`)))
    (`self.K2_DestroyActor`)
    (else
      (`KismetSystemLibrary.PrintString` "Hello"))))

(fn `UserConstructionScript`)